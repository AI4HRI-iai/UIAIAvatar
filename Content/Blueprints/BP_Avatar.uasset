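; MetaHuman-style player avatar with leader-posed body parts and Live Link ARKit subjects passed to the face AnimBP.
; When hair strands are disabled, copies eyelash opacity between dynamic materials so lower LODs show fused lashes.
; Timelines ramp turn rate as movement starts and reset it when stopped; sprint input toggles camera shake.
; Also creates a toggleable console widget, attaches the target object on overlap via C++, and provides a debug capsule-trace helper.
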(event `self.ReceiveBeginPlay`
  (bind _face (`self.Face`))
  ;[1 1 1] Console
  (`|ExecutionSequence`
    (:`then_0`
      (bind _returnvalue (`KismetSystemLibrary.GetConsoleVariableIntValue` "r.HairStrands.Strands"))
      (if (not (`KismetMathLibrary.Conv_IntToBool` _returnvalue))
        (bind _asmaterial_instance_dynamic (cast `MaterialInstanceDynamic` (`PrimitiveComponent.GetMaterial` _face 10)))
        (bind _asmaterial_instance_dynamic_2 (cast `MaterialInstanceDynamic` (`PrimitiveComponent.GetMaterial` _face 6)))
        (bind _returnvalue_2 (`MaterialInstanceDynamic.K2_GetScalarParameterValue` _asmaterial_instance_dynamic "Opacity"))
        (`MaterialInstanceDynamic.SetScalarParameterValue` _asmaterial_instance_dynamic_2 "Opacity" _returnvalue_2)
        (bind _returnvalue_3 (`MaterialInstanceDynamic.K2_GetScalarParameterValue` _asmaterial_instance_dynamic "OpacityRT"))
        (`MaterialInstanceDynamic.SetScalarParameterValue` _asmaterial_instance_dynamic_2 "OpacityRT" _returnvalue_3))
      (`self.ARKit_Setup`))
    (:`then_1`
      (bind _returnvalue_4 (`|CreateWidget` "/UIAIAvatar/Blueprints/ConsoleWidget/ConsoleWidget.ConsoleWidget_C" (`GameplayStatics.GetPlayerController` 0)))
      (set `self.ConsoleWidget` _returnvalue_4))))

(event `InputAction|ToggleConsole`
  (params (Key :type "Key Structure"))
  (bind _consolewidget (`self.ConsoleWidget`))
  ;[1 1 1] Console
  (:`Pressed`
    (if (not (`/UIAIAvatar/Blueprints/ConsoleWidget/ConsoleWidget.OpenConsole` _consolewidget))
      (`/UIAIAvatar/Blueprints/ConsoleWidget/ConsoleWidget.Open` _consolewidget))))

(event `self.ReceiveActorBeginOverlap`
  (params (OtherActor :type "Actor Object Reference"))
  (if (== OtherActor (`self.ObjectToGrasp`))
    (`self.AttachObjectCPP`)
    (`KismetSystemLibrary.PrintString` "Object Attached!")))

(event `self.ReceiveTick`
  (params (DeltaSeconds :type "Float (single-precision)"))
  (bind _charactermovement (`self.CharacterMovement`))
  (`|ExecutionSequence`
    (:`then_0`
      ;[1 1 1] Turn Rotation Speedup
      (bind _asanim_bp_avatar (cast `/UIAIAvatar/Animation_Assets/Avatar-Anim/AnimBP_Avatar` (`SkeletalMeshComponent.GetAnimInstance` (`self.Mesh`))))
      (set `self.AnimBP_Avatar` null)
      (if (> (`/UIAIAvatar/Animation_Assets/Avatar-Anim/AnimBP_Avatar.Speed` _asanim_bp_avatar) 0.01)
        (`/Engine/EditorBlueprintResources/StandardMacros.Do N` 1 :!label _label
          (:`Exit`
            (bind (_direction _increaserotationspeed) (`Timeline|RotationIncreaseFromStart` :!via `PlayFromStart`)
              (:`Update`
                (set `CharacterMovementComponent.RotationRate` (`KismetMathLibrary.MakeRotator` 0.0 0.0 _increaserotationspeed) _charactermovement)))))
        (else
          (bind (_direction_2 _rotationspeed) (`Timeline|ResetRotationSpeed`)
            (:`Update`
              (set `CharacterMovementComponent.RotationRate` (`KismetMathLibrary.MakeRotator` 0.0 0.0 _rotationspeed) _charactermovement)
              (goto _label :!via `Reset`))))))))

(event `InputAction|Sprint`
  (params (Key :type "Key Structure"))
  (bind _returnvalue (`GameplayStatics.GetPlayerCameraManager` 0))
  ;[1 1 1] Sprinting and Cam Shake
  (:`Pressed`
    (set `self.isSprinting` true)
    (if (`self.isSprinting`) :!label _label_2
      (`PlayerCameraManager.StartCameraShake` :`self` _returnvalue)
      (else
        (`PlayerCameraManager.StopAllCameraShakes` _returnvalue true))))
  (:`Released`
    (set `self.isSprinting` false)
    (goto _label_2)))

(fn `ARKit_Setup`
  (bind _asface_anim_bp (cast `/UIAIAvatar/Avatars/MetaHumans/Common/Face/Face_AnimBP` (`SkeletalMeshComponent.GetAnimInstance` (`self.Face`))))
  (set `/UIAIAvatar/Avatars/MetaHumans/Common/Face/Face_AnimBP.LLink_Face_Subj` (`self.LLink Face Subj`) _asface_anim_bp)
  (set `/UIAIAvatar/Avatars/MetaHumans/Common/Face/Face_AnimBP.LLink_Face_Head` (`self.LLink Face Head`) _asface_anim_bp))

(fn `EnableMasterPose`
  (params (SkeletalMeshComponent :type "SkeletalMeshComponent Object Reference") (Target :type "AnimMontageFactory Object Reference"))
  (if (`KismetSystemLibrary.IsValid` SkeletalMeshComponent)
    (if (not (or (`KismetSystemLibrary.IsValidClass` (`SkeletalMeshComponent.AnimClass` SkeletalMeshComponent)) (`KismetSystemLibrary.IsValidClass` (`SkeletalMesh.PostProcessAnimBlueprint` (`SkeletalMeshComponent.GetSkeletalMeshAsset` SkeletalMeshComponent)))))
      (`SkinnedMeshComponent.SetLeaderPoseComponent` SkeletalMeshComponent (`self.Mesh`) true false))))

(fn `TraceObjectsWithBP`
  (returns (ReturnValue :type "Array of HitResult Structure"))
  (bind _returnvalue (`SceneComponent.K2_GetComponentLocation` (`self.CapsuleComponent`)))
  (bind _outhits (`KismetSystemLibrary.CapsuleTraceMulti` :`Start` (- _returnvalue (0.0 0.0 10.0)) :`End` (- _returnvalue (0.0 0.0 10.099998)) :`Radius` 80.0 :`HalfHeight` 125.0 :`TraceChannel` "TraceTypeQuery1" :`DrawDebugType` "Persistent"))
  (return _outhits))

(fn `UserConstructionScript`
  (`self.EnableMasterPose` (`self.Feet`))
  (`self.EnableMasterPose` (`self.Legs`))
  (`self.EnableMasterPose` (`self.Torso`))
  (`/Engine/EditorBlueprintResources/StandardMacros.IsValid` (`self.Face`) ; Only create MIDs when there is a valid skeletal mesh is set \n(this prevents warnings in MH export)
    (:`Is Valid`
      (`PrimitiveComponent.CreateDynamicMaterialInstance` (`self.Face`) 6 null "None") ; Turn eyelashes materials into MIDs so we can toggle opacity when using hair cards
      (`PrimitiveComponent.CreateDynamicMaterialInstance` (`self.Face`) 10 null "None"))))