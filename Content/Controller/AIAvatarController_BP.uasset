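; AI controller for BP_Avatar that moves the avatar along a tagged LevelSpline or to a given location.
; StartSpline finds the spline by tag; Tick then adds movement input along its direction and snaps the avatar's XY to the nearest spline point, keeping capsule height.
; Near the spline's end, following stops and the avatar is pinned to the endpoint for two seconds.
; MoveTo separately issues a standard MoveToLocation.
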(event `self.ReceiveBeginPlay`
  (bind _asbp_avatar (cast `/UIAIAvatar/Blueprints/BP_Avatar` (`self.K2_GetPawn`)))
  (set `self.AIAvatar` _asbp_avatar))

(event `self.ReceiveTick`
  (params (DeltaSeconds :type "Float (single-precision)"))
  (if (`self.SplineRunning`)
    (`self.FollowSpline`)
    (if (not (`self.SplineRunning`))
      (set `self.StickToSpline` true)
      (`KismetSystemLibrary.Delay` 2.0)
      (set `self.StickToSpline` false))
    (elif (`self.StickToSpline`)
      (`self.StickOnSpline`))))

(fn `FollowSpline`
  (bind _spline (`/UIAIAvatar/Blueprints/AI_BP/LevelSpline.Spline` (`self.TrackRef`)))
  (bind (_returnvalue_x _returnvalue_y _returnvalue_z) (`KismetMathLibrary.BreakVector` (`SceneComponent.K2_GetComponentLocation` (`Character.CapsuleComponent` (`self.AIAvatar`)))))
  (bind _returnvalue (`SceneComponent.K2_GetComponentLocation` (`Character.Mesh` (`self.AIAvatar`))))
  (bind _returnvalue_2 (`SplineComponent.GetLocationAtDistanceAlongSpline` _spline (`SplineComponent.GetSplineLength` _spline) "World"))
  (bind _returnvalue_3 (`SplineComponent.FindLocationClosestToWorldLocation` _spline _returnvalue "World"))
  (bind _returnvalue_4 (`KismetMathLibrary.VSizeXY` (- _returnvalue_2 _returnvalue_3)))
  (if (>= _returnvalue_4 1.0)
    (`PawnMovementComponent.AddInputVector` (`Character.CharacterMovement` (`self.AIAvatar`)) (`KismetMathLibrary.GreaterGreater_VectorRotator` (`KismetMathLibrary.MakeVector` 1.0) (`SplineComponent.FindRotationClosestToWorldLocation` _spline _returnvalue "World")) false)
    (set `self.FinalPoint` _returnvalue_3)
    (else
      (set `self.SplineRunning` false)
      (`KismetSystemLibrary.PrintString` (`KismetStringLibrary.Conv_DoubleToString` _returnvalue_4))
      (set `self.FinalPoint` _returnvalue_2)))
  (`self.K2_SetActorLocation` (`self.AIAvatar`) (`KismetMathLibrary.MakeVector` (.x (`self.FinalPoint`)) (.y (`self.FinalPoint`)) _returnvalue_z) false true))

(fn `Move To`
  (params (X :type "Float (double-precision)") (Y :type "Float (double-precision)") (Z :type "Float (double-precision)"))
  (cast `/UIAIAvatar/Blueprints/BP_Avatar` (`self.K2_GetPawn`))
  (`self.MoveToLocation` (`KismetMathLibrary.MakeVector` X Y Z) 1.0 true true false true null))

(fn `StartSpline`
  (params (Spline :type Name))
  (bind _outactors (`GameplayStatics.GetAllActorsWithTag` Spline))
  (bind _aslevel_spline (cast `/UIAIAvatar/Blueprints/AI_BP/LevelSpline` (`|GetArrayItem` _outactors)))
  (set `self.TrackRef` _aslevel_spline)
  (set `self.SplineRunning` true))

(fn `StickOnSpline`
  (bind (_returnvalue_x _returnvalue_y _returnvalue_z) (`KismetMathLibrary.BreakVector` (`SceneComponent.K2_GetComponentLocation` (`Character.CapsuleComponent` (`self.AIAvatar`)))))
  (`self.K2_SetActorLocation` (`self.AIAvatar`) (`KismetMathLibrary.MakeVector` (.x (`self.FinalPoint`)) (.y (`self.FinalPoint`)) _returnvalue_z) false true))

(fn `UserConstructionScript`)